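; Game mode for Find the Kind that runs a round-based game across welcome, round and end-game widgets created at BeginPlay.
; NextRound feeds each Rounds entry to the round screen, using a resettable DoOnce for the first screen swap, then calls EndGame after the last.
; EndRound shows victory and schedules NextRound by timer.
; Tick tracks and debug-prints inactivity, returning to the welcome screen via StartGame on timeout.
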(event EventBeginPlay
  (CallFunction|InitGUI))

(event EventTick
  (params (DeltaSeconds :type Float%20%28single-precision%29))
  (bind _output_get (Variables|Default|SetInactivityTime (+ DeltaSeconds (Variables|Default|GetInactivityTime))))
  (Development|PrintString (Utilities|String|ToString(Float) _output_get) true true "(R=0.000000,G=0.660000,B=1.000000,A=1.000000)" 2.0 "dick")
  (if (> _output_get (Variables|Default|GetMaxInactivityTime))
    (CallFunction|ResetInactivityTime)
    (CallFunction|StartGame)))

(fn ConstructionScript)

(fn NextRound
  (CallFunction|ResetInactivityTime)
  (if (CallFunction|IsEndGame)
    (CallFunction|EndGame)
    (else
      (Utilities|FlowControl|Sequence
        (:then_0
          (Utilities|FlowControl|DoOnce false :!label _label
            (:Completed
              ;[1 1 1] GUI
              (Widget|RemovefromParent (Variables|GUI|GetWelcomeScreen))
              (UserInterface|Viewport|AddtoViewport (Variables|GUI|GetRoundScreen) 0))))
        (:then_1
          (Default|InitializeRoundScreen (Variables|GUI|GetRoundScreen) (Utilities|Array|Get(acopy) (Variables|Default|GetRounds) (Variables|Default|GetNextRoundId)))
          (Variables|Default|SetNextRoundId (+ (Variables|Default|GetNextRoundId) 1)))
        (:then_2
          (if (CallFunction|IsEndGame)
            (goto _label Reset)))))))

(fn IsEndGame
  (return (> (Variables|Default|GetNextRoundId) (Utilities|Array|LastIndex (Variables|Default|GetRounds)))))

(fn StartGame
  (Variables|Default|SetNextRoundId 0)
  (UserInterface|Viewport|AddtoViewport (Variables|GUI|GetWelcomeScreen) 0)
  (Utilities|FlowControl|Sequence
    (:then_0
      (Widget|RemovefromParent (Variables|GUI|GetRoundScreen)))
    (:then_1
      (Widget|RemovefromParent (Variables|GUI|GetEndGameScreen)))))

(fn EndRound
  (CallFunction|ResetInactivityTime)
  (Default|SetVisibilityVictory (Variables|GUI|GetRoundScreen))
  (Utilities|Time|SetTimerbyFunctionName 0 "NextRound" (Variables|Default|GetEndRoundPause)))

(fn EndGame
  (CallFunction|ResetInactivityTime)
  (UserInterface|Viewport|AddtoViewport (Variables|GUI|GetEndGameScreen) 0))

(fn ResetInactivityTime
  (Variables|Default|SetInactivityTime 0.0))

(fn InitGUI
  (Utilities|FlowControl|Sequence
    (:then_0
      (bind _returnvalue (UserInterface|CreateWidget "/Game/find_the_kind/gui/main_menu.main_menu_C"))
      (Variables|GUI|SetWelcomeScreen _returnvalue))
    (:then_1
      (bind _returnvalue_2 (UserInterface|CreateWidget "/Game/find_the_kind/gui/gamescreen.gamescreen_C"))
      (Variables|GUI|SetRoundScreen _returnvalue_2))
    (:then_2
      (bind _returnvalue_3 (UserInterface|CreateWidget "/Game/find_the_kind/gui/win_screen.win_screen_C"))
      (Variables|GUI|SetEndGameScreen _returnvalue_3))))